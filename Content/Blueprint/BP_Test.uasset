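; BP_Test is a score pickup with a spinning TextRender that the player's P38 pawn collects by flying into it.
; BeginPlay caches player pawn 0 as BP_P38Pawn, and Tick yaws the text by DeltaSeconds plus one, so spin speed depends on frame rate.
; When that pawn overlaps the Box, the actor increments its Score, calls UpdateScoreEvent and destroys itself.
; An UpdateScoreNow call remains unconnected.
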(event OnComponentBeginOverlap(Box)
  (params (OverlappedComponent :type Primitive%20Component%20Object%20Reference) (OtherActor :type Actor%20Object%20Reference) (OtherComp :type Primitive%20Component%20Object%20Reference) (OtherBodyIndex :type Integer) (bFromSweep :type Boolean) (SweepResult :type Hit%20Result%20Structure%20%28by%20ref%29))
  (bind _as_bp_p38pawn (Variables|Default|GetAs%20BP%20P38Pawn))
  ;[1 1 1 1 25] 스코어 변경해주는 방식은 똑같지만 위에 노드가 더 간편해보이고 깔끔하다
  (if (== OtherActor (Variables|Default|GetAs%20BP%20P38Pawn))
    (bind _output_get (Variables|/Game/Blueprint/BP_P38Pawn.BP_P38Pawn_C|SetScore _as_bp_p38pawn (+ (Variables|Default|GetScore) 1)))
    (Default|UpdateScoreEvent _as_bp_p38pawn _output_get)
    (Actor|DestroyActor)))

(event EventBeginPlay
  (bind _asbp_p38pawn (Utilities|Casting|CastToBP_P38Pawn (Game|Player|GetPlayerPawn 0)))
  (Variables|Default|SetAs%20BP%20P38Pawn _asbp_p38pawn))

(event Collision|EventActorBeginOverlap
  (params (OtherActor :type Actor%20Object%20Reference)))

(event EventTick
  (params (DeltaSeconds :type Float%20%28single-precision%29))
  ;[1 1 1 1 25] 틱마다 텍스트렌더를 회전시켜주는 노드
  (Transformation|AddLocalRotation (Variables|Default|GetTextRender) (Math|Rotator|MakeRotator 0.0 0.0 (+ DeltaSeconds 1.0)) false false))

(fn ConstructionScript)