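; BP_P38Pawn is a player-controlled P-38 plane pawn that flies forward constantly and fires rockets.
; Tick feeds full forward movement input, while Pitch and Roll axes rotate the actor locally, scaled by RotationSpeed and delta time.
; On BeginPlay it registers the Left and Right propeller components with the ACRotarionMovement component for rotation.
; Left mouse button spawns a BP_Rocket at the pawn's transform.
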(event EventBeginPlay
  ;[1 1 1] PropellerRotation
  (Utilities|Array|Add (Variables|/Game/Movement/AC_RotationMovement.AC_RotationMovement_C|GetSceneComponent (Variables|Default|GetAC_RotarionMovement)) (Variables|Default|Getleft))
  (Utilities|Array|Add (Variables|/Game/Movement/AC_RotationMovement.AC_RotationMovement_C|GetSceneComponent (Variables|Default|GetAC_RotarionMovement)) (Variables|Default|Getright)))

(event Collision|EventActorBeginOverlap
  (params (OtherActor :type Actor%20Object%20Reference)))

(event EventTick
  (params (DeltaSeconds :type Float%20%28single-precision%29))
  ;[1 1 1] PawnFowardMovement
  (Pawn|Input|AddMovementInput (Transformation|GetActorForwardVector) 1.0 false))

(event Input|AxisEvents|InputAxisPitch
  (params (AxisValue :type Float%20%28single-precision%29))
  ;[1 1 1] PawnUp,DownMovement
  (Transformation|AddActorLocalRotation (Math|Rotator|MakeRotator 0.0 (* AxisValue (Utilities|Time|GetWorldDeltaSeconds) (Variables|Default|GetRotationSpeed)) 0.0) false false))

(event Input|AxisEvents|InputAxisRoll
  (params (AxisValue :type Float%20%28single-precision%29))
  ;[1 1 1] PawnLeft,RightMovement
  (Transformation|AddActorLocalRotation (Math|Rotator|MakeRotator (* AxisValue (Utilities|Time|GetWorldDeltaSeconds) (Variables|Default|GetRotationSpeed)) 0.0 0.0) false false))

(event Input|MouseEvents|LeftMouseButton
  (params (Key :type Key%20Structure :default "None"))
  ;[1 1 1] RocketSpawn
  (:Pressed
    (Game|SpawnActorfromClass "/Game/Blueprint/BP_Rocket.BP_Rocket_C" (Transformation|GetActorTransform) "Undefined" "MultiplyWithRoot" 0 0)))

(fn ConstructionScript)