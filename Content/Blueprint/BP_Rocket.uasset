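; BP_Rocket is a rocket actor with a limited lifespan and particle effects for launch and impact.
; On BeginPlay it attaches a particle effect and a brief small fire burst to its mesh.
; Any actor overlap spawns sparks at its location, then after a delay removes them, calls a sound spawn with no sound asset shown, and destroys the rocket.
; The Blueprint graphs contain no movement or damage logic.
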(event EventBeginPlay
  (Utilities|FlowControl|Sequence
    (:then_0
      (Effects|SpawnEmitterAttached "/Engine/Tutorial/SubEditors/TutorialAssets/TutorialParticleSystem.TutorialParticleSystem" (Variables|Default|GetStaticMesh) "None")
      (Actor|SetLifeSpan 5.0))
    (:then_1
      (bind _returnvalue (Effects|SpawnEmitterAttached "/Game/StarterContent/Particles/P_Fire.P_Fire" (Variables|Default|GetStaticMesh) "None" "0, 0, 0" "0, 0, 0" "0.200000,0.200000,0.200000"))
      (Utilities|FlowControl|Delay 0.2)
      (Components|DestroyComponent _returnvalue))))

(event Collision|EventActorBeginOverlap
  (params (OtherActor :type Actor%20Object%20Reference))
  ;[1 1 1 1 35] 로켓 디스트로이
  ;;[1 1 1 1 25] 이미터를 생성하고 1초뒤에 디스트로이 시킨다
  (bind _returnvalue (Effects|SpawnEmitteratLocation "/Game/StarterContent/Particles/P_Sparks.P_Sparks" (Transformation|GetActorLocation)))
  (Utilities|FlowControl|Delay 1.0)
  (Components|DestroyComponent _returnvalue)
  ;;[1 1 1 1 25] 사운드를 생성하고 로켓을 디스트로이 한다
  (Audio|SpawnSoundatLocation 0 (Transformation|GetActorLocation) "0, 0, 0" 1.0 1.0 0.0 0 0)
  (Actor|DestroyActor))

(event EventTick
  (params (DeltaSeconds :type Float%20%28single-precision%29)))

(fn ConstructionScript)